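; Trigger volume that switches the player's camera view while the Tino_BP character is inside it.
; On overlap begin, it gets the character's PlayerController and blends the view target to the CameraToFind reference.
; On overlap end, it calls the same blend with no target set, releasing that camera.
; Both transitions share the CameraBlendTime variable, and other actors are ignored through the cast.
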(event `self.OverlapVolume.OnComponentBeginOverlap`
  (params (OverlappedComponent :type "PrimitiveComponent Object Reference") (OtherActor :type "Actor Object Reference") (OtherComp :type "PrimitiveComponent Object Reference") (OtherBodyIndex :type Integer) (bFromSweep :type Boolean) (SweepResult :type "HitResult Structure (by ref)"))
  (bind _astino_bp (cast `/Game/Tino/Tino_BP` OtherActor))
  (if (`KismetSystemLibrary.IsValid` _astino_bp)
    (bind _asplayer_controller (cast `PlayerController` (`Pawn.GetController` _astino_bp)))
    (if (`KismetSystemLibrary.IsValid` _asplayer_controller)
      (`PlayerController.SetViewTargetWithBlend` _asplayer_controller (`self.CameraToFind`) (`self.CameraBlendTime`) "VTBlend_Linear" 0.0 false))))

(event `self.OverlapVolume.OnComponentEndOverlap`
  (params (OverlappedComponent :type "PrimitiveComponent Object Reference") (OtherActor :type "Actor Object Reference") (OtherComp :type "PrimitiveComponent Object Reference") (OtherBodyIndex :type Integer))
  (bind _astino_bp (cast `/Game/Tino/Tino_BP` OtherActor))
  (if (`KismetSystemLibrary.IsValid` _astino_bp)
    (bind _asplayer_controller (cast `PlayerController` (`Pawn.GetController` _astino_bp)))
    (if (`KismetSystemLibrary.IsValid` _asplayer_controller)
      (`PlayerController.SetViewTargetWithBlend` _asplayer_controller null (`self.CameraBlendTime`) "VTBlend_Linear" 0.0 false))))

(fn `UserConstructionScript`)